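; BP_BasiAI is a basic AI pawn that continuously wanders the navmesh.
; On Tick, when IsMoving is false, AI MoveTo sends it to a random navigable point within a fixed radius of its mesh's current location.
; IsMoving blocks new requests during a move and clears on success or failure, so the next Tick picks another destination.
; A SimpleMoveToLocation node is left unconnected and never runs.
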(event EventBeginPlay)

(event Collision|EventActorBeginOverlap
  (params (OtherActor :type Actor%20Object%20Reference)))

(event EventTick
  (params (DeltaSeconds :type Float%20%28single-precision%29))
  (bind _self self)
  (if (not (Variables|Default|GetisMoving))
    (AI|AIMoveTo _self (.RandomLocation (Class|NavigationSystem|GetRandomPointinNavigableRadius (Transformation|GetWorldLocation (Variables|Character|GetMesh _self)) 1e+03)) 0 5.0 false
      (:then
        (Variables|Default|SetisMoving true))
      (:OnSuccess
        (Variables|Default|SetisMoving false :!label _label))
      (:OnFail
        (goto _label)))))

(fn ConstructionScript)