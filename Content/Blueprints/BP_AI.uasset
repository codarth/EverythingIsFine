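; BP_AI is an AI pawn that wanders at random and can be switched to ragdoll or set on fire.
; While not ragdolled, Tick starts a move to a random navigable point near the mesh whenever none is running, clearing IsMoving on success or failure.
; SetRagDoll sets the flag and stops mesh animation, and Tick then applies physics simulation every frame.
; LightOnFire flags the pawn and adds a P_Fire particle component.
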(event EventTick
  (params (DeltaSeconds :type Float%20%28single-precision%29))
  (bind _self self)
  ;[1 1 1] InRagdoll?
  (if (Variables|Default|GetinRagdoll)
    ;[1 1 1] Ragdoll Effect
    (Class|SkeletalMeshComponent|SetAllBodiesSimulatePhysics (Variables|Character|GetMesh) true)
    (Variables|Default|SetinRagdoll true)
    (else
      ;[1 1 1] Random Movement
      (if (not (Variables|Default|GetisMoving))
        (AI|AIMoveTo _self (.RandomLocation (Class|NavigationSystem|GetRandomPointinNavigableRadius (Transformation|GetWorldLocation (Variables|Character|GetMesh _self)) 1e+03)) 0 5.0 false
          (:then
            (Variables|Default|SetisMoving true))
          (:OnSuccess
            (Variables|Default|SetisMoving false :!label _label))
          (:OnFail
            (goto _label)))))))

(fn ConstructionScript)

(fn SetRagDoll
  (params (ragDoll :type Boolean))
  (Variables|Default|SetinRagdoll ragDoll)
  (Audio|Components|Audio|Stop (Variables|Character|GetMesh)))

(fn LightonFire
  (Variables|Default|SetonFire true)
  (bind _returnvalue (AddComponent|AddParticleSystemComponent false))
  (Effects|Components|ParticleSystem|SetTemplate _returnvalue "/Game/StarterContent/Particles/P_Fire.P_Fire"))