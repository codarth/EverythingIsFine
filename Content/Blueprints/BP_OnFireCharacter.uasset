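; First-person player character that lets the player light and extinguish fires and act on AI pawns.
; Each input action fires a debug-drawn line trace forward from the camera, with a range that varies by action.
; Visibility traces call set-on-fire or extinguish on BP_Burn actors.
; Pawn object traces either ragdoll a BP_AI with a slap or light it on fire.
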(event Input|ActionEvents|InputActionLightAi
  (params (Key :type Key%20Structure))
  (bind _firstpersoncameracomponent (Variables|Default|GetFirstPersonCameraComponent))
  (bind _returnvalue (Transformation|GetWorldLocation _firstpersoncameracomponent))
  (:Pressed
    (bind _outhit (Collision|LineTraceForObjects _returnvalue (+ _returnvalue (* (Math|Vector|GetForwardVector (Transformation|GetWorldRotation _firstpersoncameracomponent)) 1.5e+03)) (Utilities|Array|MakeArray "ObjectTypeQuery3") false 0 "ForDuration" true "(R=1.000000,G=0.401903,B=0.000000,A=1.000000)"))
    (bind _asbp_ai (Utilities|Casting|CastToBP_AI (.HitActor (Collision|BreakHitResult _outhit))))
    (Default|LightonFire _asbp_ai)))

(event Input|ActionEvents|InputActionSlapAI
  (params (Key :type Key%20Structure))
  (bind _firstpersoncameracomponent (Variables|Default|GetFirstPersonCameraComponent))
  (bind _returnvalue (Transformation|GetWorldLocation _firstpersoncameracomponent))
  ;[1 1 1] Slap
  (:Pressed
    (bind _outhit (Collision|LineTraceForObjects _returnvalue (+ _returnvalue (* (Math|Vector|GetForwardVector (Transformation|GetWorldRotation _firstpersoncameracomponent)) 1.5e+03)) (Utilities|Array|MakeArray "ObjectTypeQuery3") false 0 "ForDuration" true "(R=1.000000,G=0.401903,B=0.000000,A=1.000000)"))
    (bind _asbp_ai (Utilities|Casting|CastToBP_AI (.HitActor (Collision|BreakHitResult _outhit))))
    (Default|SetRagDoll _asbp_ai true)))

(event Input|ActionEvents|InputActionExtinguishFire
  (params (Key :type Key%20Structure))
  (bind _firstpersoncameracomponent (Variables|Default|GetFirstPersonCameraComponent))
  (bind _returnvalue (Transformation|GetWorldLocation _firstpersoncameracomponent))
  ;[1 1 1] Extinguish Fire
  (:Pressed
    (bind _outhit (Collision|LineTraceByChannel _returnvalue (+ _returnvalue (* (Math|Vector|GetForwardVector (Transformation|GetWorldRotation _firstpersoncameracomponent)) 1e+03)) "TraceTypeQuery1" false 0 "ForDuration"))
    (bind _asbp_burn (Utilities|Casting|CastToBP_Burn (.HitActor (Collision|BreakHitResult _outhit))))
    (Default|ExtinguishFire _asbp_burn)))

(event Input|ActionEvents|InputActionLightFire
  (params (Key :type Key%20Structure))
  (bind _firstpersoncameracomponent (Variables|Default|GetFirstPersonCameraComponent))
  (bind _returnvalue (Transformation|GetWorldLocation _firstpersoncameracomponent))
  ;[1 1 1] LightFire
  (:Pressed
    (bind _outhit (Collision|LineTraceByChannel _returnvalue (+ _returnvalue (* (Math|Vector|GetForwardVector (Transformation|GetWorldRotation _firstpersoncameracomponent)) 5e+02)) "TraceTypeQuery1" false 0 "ForDuration" true "(R=1.000000,G=0.812642,B=0.000000,A=1.000000)"))
    (bind _asbp_burn (Utilities|Casting|CastToBP_Burn (.HitActor (Collision|BreakHitResult _outhit))))
    (Default|SetonFire _asbp_burn)))

(fn ConstructionScript)