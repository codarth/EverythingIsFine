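; BP_Burn is a flammable actor that catches fire when a BP_AI hits it.
; On hit it sets IsOnFire, starts the Flames component's trails, moves it to the hit location and assigns the Fire particle template.
; BeginPlay randomizes an integer-valued BurnTime, which nothing here reads.
; ExtinguishFire clears the flag and ends the trails, but is not called within this Blueprint.
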(event EventBeginPlay
  ;[1 1 1] Set Random Burn Time
  (Variables|Default|SetBurnTime (Math|Conversions|ToFloat(Integer) (Math|Random|RandomIntegerinRange 10 30))))

(event Collision|EventHit
  (params (MyComp :type Primitive%20Component%20Object%20Reference) (Other :type Actor%20Object%20Reference) (OtherComp :type Primitive%20Component%20Object%20Reference) (bSelfMoved :type Boolean) (HitLocation :type Vector :default "0, 0, 0") (HitNormal :type Vector :default "0, 0, 0") (NormalImpulse :type Vector :default "0, 0, 0") (Hit :type Hit%20Result%20Structure%20%28by%20ref%29))
  (bind _flames (Variables|Default|Getflames))
  ;[1 1 1] Light Fire on AI Hit
  (Utilities|Casting|CastToBP_AI Other)
  (CallFunction|SetonFire)
  (Transformation|SetWorldLocation _flames HitLocation false false)
  (Effects|Components|ParticleSystem|SetTemplate _flames "/Game/Particles/Fire.Fire"))

(fn ConstructionScript)

(fn SetonFire
  (Variables|Default|SetisOnFire true)
  (Effects|Particles|Trails|BeginTrails (Variables|Default|GetFlames) "None" "None" "ETrailWidthMode_FromCentre" 0.0))

(fn ExtinguishFire
  (Variables|Default|SetisOnFire false)
  (Effects|Particles|Trails|EndTrails (Variables|Default|GetFlames)))